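; Gameplay ability for the player's first melee punch, built on a parent ability's activation logic.
; It plays the punch montage with a combo-trigger event tag and ends when the montage completes, blends out or is interrupted or cancelled.
; It also waits for combo window begin, then end events, though nothing follows them here.
; The avatar's input cache is cleared on activation and on end.
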(event Ability|EventActivateAbility
  (|CallParentFunction)
  (Default|ClearInputCache (Variables|Default|GetAvatarCharacter))
  (|PlayMontageandWaitforEvent "None" (Variables|Setting|GetMontage) "(GameplayTags=((TagName=\"Event.Character.CanTriggerCombo\")))" (Variables|Setting|GetPlayRate) "None" true 1.0
    (:then
      (Ability|Tasks|WaitGameplayEvent "(TagName=\"Event.Character.ComboWindowBegin\")" 0
        (:then
          (Ability|Tasks|WaitGameplayEvent "(TagName=\"Event.Character.ComboWindowEnd\")" 0))))
    (:OnCompleted
      (Ability|EndAbility :!label _label))
    (:OnBlendOut
      (goto _label))
    (:OnInterrupted
      (goto _label))
    (:OnCancelled
      (goto _label))))

(event Ability|EventOnEndAbility
  (params (bWasCancelled :type Boolean))
  (Default|ClearInputCache (Variables|Default|GetAvatarCharacter)))