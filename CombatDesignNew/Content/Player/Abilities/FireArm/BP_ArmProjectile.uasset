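; Fired-arm projectile for the player's FireArm ability, which teleports the player to where it hits.
; It flies for a limited lifespan, and overlaps with characters other than the Golem boss are ignored.
; Any other overlap stops it, clears its lifespan, plays hit sound and Niagara effect, then calls TeleportToArm on the player after a short delay.
; On destruction it notifies the player through OnArmProjectileDestroyed.
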(event OnComponentBeginOverlap(Collision)
  (params (OverlappedComponent :type Primitive%20Component%20Object%20Reference) (OtherActor :type Actor%20Object%20Reference) (OtherComp :type Primitive%20Component%20Object%20Reference) (OtherBodyIndex :type Integer) (bFromSweep :type Boolean) (SweepResult :type Hit%20Result%20Structure%20%28by%20ref%29))
  (bind _ns_fisthit (Variables|Default|GetNS_FistHit))
  (Utilities|Casting|CastToCharacter OtherActor
    (:then
      (Utilities|Casting|CastToBP_Enemy_GolemBoss OtherActor))
    (:CastFailed
      _))
  (Game|Components|ProjectileMovement|SetVelocityinLocalSpace (Variables|Default|GetProjectileMovement) "0, 0, 0")
  (Actor|SetLifeSpan 0.0)
  (Audio|PlaySound2D "/Game/SFX/Fist_Hit.Fist_Hit" 1.0 1.0 0.0 0 0)
  (Niagara|ResetSystem _ns_fisthit)
  (Components|Activation|Activate _ns_fisthit false)
  (Utilities|FlowControl|Delay 0.3)
  (bind _returnvalue (Actor|GetActorOfClass "/Game/Player/BP_PlayerCharacter.BP_PlayerCharacter_C"))
  (Default|TeleporttoArm _returnvalue self))

(event EventBeginPlay
  (Actor|SetLifeSpan (Variables|Default|GetProjectileLifespan))
  (Components|Activation|ToggleActive (Variables|Default|GetNS_FistHit)))

(event EventDestroyed
  (bind _returnvalue (Actor|GetActorOfClass "/Game/Player/BP_PlayerCharacter.BP_PlayerCharacter_C"))
  (Default|OnArmProjectileDestroyed _returnvalue))

(fn ConstructionScript)