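; BP_DamageFlash is a component that briefly flashes its owner's skeletal mesh when the owner takes damage.
; On BeginPlay it binds to OnTakeAnyDamage, creates a dynamic material instance on the first material slot and caches the original emissive color.
; DamageFlash sets the emissive color and multiplier, then restores them after a short delay.
; The multiplier caching is disconnected, so the restore uses that variable's unmodified value.
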(event Custom|DamageFlash
  (params (DamagedActor :type Actor%20Object%20Reference) (Damage :type Float%20%28single-precision%29) (DamageType :type Damage%20Type%20Object%20Reference) (InstigatedBy :type Controller%20Object%20Reference) (DamageCauser :type Actor%20Object%20Reference))
  (bind _flashmat (Variables|Default|GetFlashMat))
  (bind _flashmat_2 (Variables|Default|GetFlashMat))
  (Rendering|Material|SetVectorParameterValue _flashmat_2 "EmissiveColor" (Variables|Default|GetFlashCDolor) :!class /Script/Engine.MaterialInstanceDynamic)
  (Rendering|Material|SetScalarParameterValue _flashmat_2 "EmissiveMultiplyer" 1.0 :!class /Script/Engine.MaterialInstanceDynamic)
  (Utilities|FlowControl|Delay 0.2)
  (Rendering|Material|SetVectorParameterValue _flashmat "EmissiveColor" (Variables|Default|GetInetEmissiveColor) :!class /Script/Engine.MaterialInstanceDynamic)
  (Rendering|Material|SetScalarParameterValue _flashmat "EmissiveMultiplyer" (Variables|Default|GetInetEmissiveMultiplyer) :!class /Script/Engine.MaterialInstanceDynamic))

(event EventBeginPlay
  (bind _returnvalue (Components|GetOwner))
  (Variables|Default|SetOwner _returnvalue)
  (EventDispatchers|BindEventtoOnTakeAnyDamage _returnvalue (EventDispatchers|CreateEvent :!event Custom|DamageFlash))
  (Utilities|IsValid (Actor|GetComponentbyClass (Variables|Default|GetOwner) "/Script/Engine.SkeletalMeshComponent")
    (:Is%20Valid
      (bind _returnvalue_2 (Rendering|Material|CreateDynamicMaterialInstance (Actor|GetComponentbyClass (Variables|Default|GetOwner) "/Script/Engine.SkeletalMeshComponent") 0 0 "None" :!class /Script/Engine.PrimitiveComponent))
      (Variables|Default|SetFlashMat _returnvalue_2)
      (bind _returnvalue_3 (Rendering|Material|GetVectorParameterValue (Variables|Default|GetFlashMat) "EmissiveColor" :!class /Script/Engine.MaterialInstanceDynamic))
      (Variables|Default|SetInetEmissiveColor _returnvalue_3))))

(event EventTick
  (params (DeltaSeconds :type Float%20%28single-precision%29)))