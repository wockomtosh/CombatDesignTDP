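; Enemy weak point actor that periodically toggles between exposed and invulnerable, swapping its mesh material to show the state.
; While exposed, TakeDamage lowers HP, fires a damage event and flickers the material through chained delays.
; At zero HP it fires a destroyed event and shows a broken mesh instead of destroying the actor.
; Character overlap with the collision deals one damage as a test hook.
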(event OnComponentBeginOverlap(Collision)
  (params (OverlappedComponent :type Primitive%20Component%20Object%20Reference) (OtherActor :type Actor%20Object%20Reference) (OtherComp :type Primitive%20Component%20Object%20Reference) (OtherBodyIndex :type Integer) (bFromSweep :type Boolean) (SweepResult :type Hit%20Result%20Structure%20%28by%20ref%29))
  ;[0.15 0.15 0.15 0.5] For testing
  (Utilities|Casting|CastToCharacter OtherActor)
  (CallFunction|TakeDamage 1.0))

(event Custom|TakeDamage
  (params (Damage :type Float%20%28double-precision%29))
  (if (not (Variables|Default|GetDestroyed))
    (if (Variables|Default|GetExposed)
      (bind _output_get (Variables|Default|SetCurrentHP (- (Variables|Default|GetCurrentHP) Damage)))
      (Default|CallOnDamageTaken Damage)
      (CallFunction|DamageTakenEffect)
      (if (<= _output_get 0.0)
        (CallFunction|WeakPointDestroyed))
      (else
        (Development|PrintString "Weak point is invulnerable")))))

(event Custom|WeakPointDestroyed
  ;[0.15 0.15 0.15 0.5] I'm not tying this to the actor destroyed event because we may want the weak spot to still show up but look "Broken"
  (Default|CallOnWeakPointDestroyed)
  (Development|SetHiddeninGame (Variables|Default|GetDestroyedMesh) false false)
  (Development|SetHiddeninGame (Variables|Default|GetRegularMesh) true false)
  (Variables|Default|SetDestroyed true))

(event Custom|Expose
  (Variables|Default|SetExposed true)
  (Rendering|Material|SetMaterial (Variables|Default|GetRegularMesh) 0 "/Game/Player/Assets/Material/M_Eyes.M_Eyes"))

(event Custom|Hide
  (Variables|Default|SetExposed false)
  (Rendering|Material|SetMaterial (Variables|Default|GetRegularMesh) 0 "/Game/EngineDefault/StarterContent/Props/Materials/M_Frame.M_Frame"))

(event Custom|DamageTakenEffect
  (Rendering|Material|SetMaterial (Variables|Default|GetRegularMesh) 0 "/Game/Player/Assets/Material/M_Body.M_Body")
  (Utilities|FlowControl|Delay (Variables|Default|GetDamageColorChangeDelay))
  (if (Variables|Default|GetExposed)
    (Rendering|Material|SetMaterial (Variables|Default|GetRegularMesh) 0 "/Game/Player/Assets/Material/M_Eyes.M_Eyes")
    (Utilities|FlowControl|Delay (Variables|Default|GetDamageColorChangeDelay))
    (if (Variables|Default|GetExposed)
      (Rendering|Material|SetMaterial (Variables|Default|GetRegularMesh) 0 "/Game/Player/Assets/Material/M_Body.M_Body")
      (Utilities|FlowControl|Delay (Variables|Default|GetDamageColorChangeDelay))
      (if (Variables|Default|GetExposed)
        (Rendering|Material|SetMaterial (Variables|Default|GetRegularMesh) 0 "/Game/Player/Assets/Material/M_Eyes.M_Eyes")))))

(event EventBeginPlay
  (Variables|Default|SetCurrentHP (Variables|Default|GetMaxHP))
  (CallFunction|Hide))

(event EventTick
  (params (DeltaSeconds :type Float%20%28single-precision%29))
  ;[0.15 0.15 0.15 0.5] For testing
  (bind _output_get (Variables|Default|SetExposedTimer (+ DeltaSeconds (Variables|Default|GetExposedTimer))))
  (if (>= _output_get (Variables|Default|GetExposedInterval))
    (Variables|Default|SetExposedTimer 0.0)
    (if (Variables|Default|GetExposed)
      (CallFunction|Hide)
      (else
        (CallFunction|Expose)))))

(fn ConstructionScript)