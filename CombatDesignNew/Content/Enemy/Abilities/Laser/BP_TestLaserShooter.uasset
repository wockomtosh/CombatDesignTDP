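; BP_TestLaserShooter is a test laser enemy actor that turns to face the player; no firing logic appears in this Blueprint.
; It caches player pawn 0 on BeginPlay.
; Each Tick, while that pawn is valid, it uses RInterpTo to rotate the root toward it, with Delay as interp speed, so higher values track faster.
; An unconnected variant snaps instantly to the target and never runs.
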(event EventBeginPlay
  (Variables|Default|SetCharacter (Game|Player|GetPlayerPawn 0)))

(event EventTick
  (params (DeltaSeconds :type Float%20%28single-precision%29))
  (bind _character (Variables|Default|GetCharacter))
  (Utilities|IsValid _character
    (:Is%20Valid
      ;[0.15 0.15 0.15 0.5] Look at Player in realtime with a delay
      (Transformation|SetWorldRotation (Variables|Default|GetDefaultSceneRoot) (Math|Interpolation|RInterpTo (Transformation|GetWorldRotation (Variables|Default|GetDefaultSceneRoot)) (Math|Rotator|FindLookatRotation (Transformation|GetActorLocation) (Transformation|GetActorLocation _character)) (Utilities|Time|GetWorldDeltaSeconds) (Variables|Default|GetDelay)) false false))))

(fn ConstructionScript)