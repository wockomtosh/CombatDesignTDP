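; BP_Laser is an enemy laser ability actor that repeatedly hurts the player character while they overlap its Cube component.
; Cube overlap events cache the player and toggle the OnHurt flag, which Tick checks.
; While the flag is set, a Delay in Tick throttles a State.Character.OnHurt gameplay event sent to the player, with a fixed magnitude as payload.
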(event OnComponentBeginOverlap(Cube)
  (params (OverlappedComponent :type Primitive%20Component%20Object%20Reference) (OtherActor :type Actor%20Object%20Reference) (OtherComp :type Primitive%20Component%20Object%20Reference) (OtherBodyIndex :type Integer) (bFromSweep :type Boolean) (SweepResult :type Hit%20Result%20Structure%20%28by%20ref%29))
  (bind _asbp_player_character (Utilities|Casting|CastToBP_PlayerCharacter OtherActor))
  (Variables|Default|SetPlayer%20Character _asbp_player_character)
  (Variables|Default|SetOnHurt true))

(event OnComponentEndOverlap(Cube)
  (params (OverlappedComponent :type Primitive%20Component%20Object%20Reference) (OtherActor :type Actor%20Object%20Reference) (OtherComp :type Primitive%20Component%20Object%20Reference) (OtherBodyIndex :type Integer))
  (Variables|Default|SetOnHurt false))

(event EventTick
  (params (DeltaSeconds :type Float%20%28single-precision%29))
  (if (Variables|Default|GetOnHurt)
    (Utilities|FlowControl|Delay 0.2)
    (Ability|SendGameplayEventtoActor (Variables|Default|GetPlayer%20Character) "(TagName=\"State.Character.OnHurt\")" (Utilities|Struct|MakeGameplayEventData "(TagName=\"State.Character.OnHurt\")" 0 0 0 0 "()" "(GameplayTags=)" "(GameplayTags=)" 5.0))))

(fn ConstructionScript)