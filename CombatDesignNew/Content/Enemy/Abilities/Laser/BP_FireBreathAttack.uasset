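; BP_FireBreathAttack is an enemy fire breath hazard that sphere-traces for pawns every tick from BeginPlay, ignoring its parent actor.
; A hit player character receives a Launched gameplay event carrying the hit result as target data, with debug drawing showing the trace and hit.
; The ActivateAttack timeline meant to toggle the attack never runs, and the trace endpoint helper's Arrow-based calculation is left unconnected.
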(event EventBeginPlay
  (Variables|Default|SetOriginLocation (Transformation|GetWorldLocation (Variables|Default|GetDefaultSceneRoot)))
  (Variables|Default|SetIsActive true))

(event EventTick
  (params (DeltaSeconds :type Float%20%28single-precision%29))
  (bind (_startlocation _endlocation) (|GetStartEndLocation_2))
  (if (Variables|Default|GetIsActive)
    (bind (_outhit _returnvalue) (Collision|SphereTraceForObjects _startlocation _endlocation (Variables|Default|GetRadius) (Utilities|Array|MakeArray "ObjectTypeQuery3") false (Utilities|Array|MakeArray (Actor|GetParentActor)) "ForOneFrame" true "(R=1.000000,G=0.000000,B=0.000000,A=1.000000)" "(R=0.000000,G=1.000000,B=0.000000,A=1.000000)" 0.0))
    (if _returnvalue
      (bind _asbp_player_character (Utilities|Casting|CastToBP_PlayerCharacter (.HitActor (Collision|BreakHitResult _outhit))))
      (Ability|SendGameplayEventtoActor _asbp_player_character "(TagName=\"Event.Character.Launched\")" (Utilities|Struct|MakeGameplayEventData "(TagName=\"Event.Character.Launched\")" 0 _asbp_player_character 0 0 "()" "(GameplayTags=)" "(GameplayTags=)" 0.0 (Ability|TargetData|AbilityTargetDatafromHitResult _outhit)))
      (Rendering|Debug|DrawDebugSphere (.Location (Collision|BreakHitResult _outhit)) 3e+01 12 "(R=1.000000,G=0.612561,B=0.000000,A=1.000000)" 2.0))))

(fn ConstructionScript)