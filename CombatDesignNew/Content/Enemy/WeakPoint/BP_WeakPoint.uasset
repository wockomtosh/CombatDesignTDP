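; Destructible boss weak point with its own GAS health, set at BeginPlay through a SetByCaller effect.
; GSCCore damage is forwarded to the instigating BP_BossEnemy as gameplay events, capped to the weak point's remaining health.
; Death swaps to the destroyed mesh, updates state tags and sends bonus damage to the boss.
; A test timeline sends Expose/Hide events, debug text shows health, and older non-GAS damage logic remains archived.
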(event OnDeath(GSCCore)
  (bind _returnvalue (Game|GetInstigator))
  (CallFunction|StartDeathRoutine)
  ;[0.15 0.15 0.15 0.5] Change weakpoint state
  (Ability|GameplayEffect|AddLooseGameplayTags self (GameplayTags|MakeLiteralGameplayTagContainer "(GameplayTags=((TagName=\"State.Enemy.WeakPoint.Destroyed\")))"))
  (Ability|GameplayEffect|RemoveLooseGameplayTags self (GameplayTags|MakeLiteralGameplayTagContainer "(GameplayTags=((TagName=\"State.Enemy.WeakPoint.Exposed\"),(TagName=\"State.Enemy.WeakPoint.Hidden\")))"))
  ;[0.15 0.15 0.15 0.5] Hide debug text
  (Development|SetHiddeninGame (Variables|Default|GetExposeTextDebug) true false)
  ;[0.15 0.15 0.15 0.5] Send extra damage data to enemy
  (bind _asbp_boss_enemy (Utilities|Casting|CastToBP_BossEnemy _returnvalue))
  (Utilities|IsValid _asbp_boss_enemy
    (:Is%20Valid
      (Ability|SendGameplayEventtoActor _asbp_boss_enemy "(TagName=\"Event.Enemy.WeakPoint.OnDestroy\")" (Utilities|Struct|MakeGameplayEventData "(TagName=\"\")" 0 _returnvalue 0 0 "()" "(GameplayTags=)" "(GameplayTags=)" (Variables|Setting|GetDestructionExtraDamage))))))

(event OnDamage(GSCCore)
  (params (DamageAmount :type Float%20%28single-precision%29) (SourceCharacter :type Actor%20Object%20Reference) (DamageTags :type Gameplay%20Tag%20Container%20Structure%20%28by%20ref%29))
  (bind _returnvalue (Game|GetInstigator))
  ;[0.15 0.15 0.15 0.5] Send damage data to enemy
  (bind _asbp_boss_enemy (Utilities|Casting|CastToBP_BossEnemy _returnvalue))
  (Utilities|IsValid _asbp_boss_enemy
    (:Is%20Valid
      (Ability|SendGameplayEventtoActor _asbp_boss_enemy "(TagName=\"Event.Enemy.WeakPoint.OnHit\")" (Utilities|Struct|MakeGameplayEventData "(TagName=\"\")" SourceCharacter _returnvalue 0 0 "()" "(GameplayTags=)" "(GameplayTags=)" (Math|Float|Clamp(Float) DamageAmount 0.0 (Variables|Default|GetDamageCap))))
      ;[0.15 0.15 0.15 0.5] Sent damage cannot be larger than remaining health
      (Variables|Default|SetDamageCap (.ReturnValue (Ability|Attribute|GetFloatAttribute self "(AttributeName=\"Health\",Attribute=/Script/GASCompanion.GSCAttributeSet:Health,AttributeOwner=\"/Script/CoreUObject.Class'/Script/GASCompanion.GSCAttributeSet'\")"))))))

(event Custom|TakeDamage
  (params (Damage :type Float%20%28double-precision%29))
  ;[0.15 0.15 0.15 0.5] Archived
  (if (not (Variables|Archived|GetDestroyed))
    (if (Variables|Archived|GetExposed)
      (bind _output_get (Variables|Archived|SetCurrentHP (- (Variables|Archived|GetCurrentHP) Damage)))
      (Default|CallOnDamageTaken Damage)
      (CallFunction|DamageTakenEffect)
      (if (<= _output_get 0.0)
        (CallFunction|WeakPointDestroyed))
      (else
        (Development|PrintString "Weak point is invulnerable")))))

(event Custom|WeakPointDestroyed
  ;[0.15 0.15 0.15 0.5] Archived
  ;;[0.15 0.15 0.15 0.5] I'm not tying this to the actor destroyed event because we may want the weak spot to still show up but look "Broken"
  (Default|CallOnWeakPointDestroyed))

(event Custom|Expose
  ;[0.15 0.15 0.15 0.5] Archived
  (Variables|Archived|SetExposed true)
  (Rendering|Material|SetMaterial (Variables|Default|GetMesh) 0 "/Game/Player/Assets/Material/M_Eyes.M_Eyes"))

(event Custom|Hide
  ;[0.15 0.15 0.15 0.5] Archived
  (Variables|Archived|SetExposed false)
  (Rendering|Material|SetMaterial (Variables|Default|GetMesh) 0 "/Game/EngineDefault/StarterContent/Props/Materials/M_Frame.M_Frame"))

(event Custom|DamageTakenEffect
  ;[0.15 0.15 0.15 0.5] Archived
  (Rendering|Material|SetMaterial (Variables|Default|GetMesh) 0 "/Game/Enemy/WeakPoint/Material/M_Damage.M_Damage")
  (Utilities|FlowControl|Delay (Variables|Archived|GetDamageColorChangeDelay))
  (if (Variables|Archived|GetExposed)
    (Rendering|Material|SetMaterial (Variables|Default|GetMesh) 0 "/Game/Player/Assets/Material/M_Eyes.M_Eyes")
    (Utilities|FlowControl|Delay (Variables|Archived|GetDamageColorChangeDelay))
    (if (Variables|Archived|GetExposed)
      (Rendering|Material|SetMaterial (Variables|Default|GetMesh) 0 "/Game/Enemy/WeakPoint/Material/M_Damage.M_Damage")
      (Utilities|FlowControl|Delay (Variables|Archived|GetDamageColorChangeDelay))
      (if (Variables|Archived|GetExposed)
        (Rendering|Material|SetMaterial (Variables|Default|GetMesh) 0 "/Game/Player/Assets/Material/M_Eyes.M_Eyes")))))

(event EventBeginPlay
  (bind _maxhealth (Variables|Setting|GetMaxHealth))
  (Utilities|FlowControl|Sequence
    (:then_0
      (CallFunction|SetMaxHealth _maxhealth)
      (Variables|Default|SetDamageCap _maxhealth))
    (:then_1
      ;[0.15 0.15 0.15 0.5] Testing
      (bind _time (Timeline|TestStatusSwitchingByEvent Play)
        (:Update
          (Rendering|Components|TextRender|SetText (Variables|Default|GetExposeTextDebug) (Utilities|Text|ToText(Float) (Math|Float|%(Float) _time 5.0) "FromZero" false true 1 1 0 0)))
        (:Expose
          ;[0.15 0.15 0.15 0.5] Methods to trigger status switching: By sending Gameplay Events to BP_WeakPoint
          (Ability|SendGameplayEventtoActor self "(TagName=\"Event.Enemy.WeakPoint.Expose\")"))
        (:Hide
          (Ability|SendGameplayEventtoActor self "(TagName=\"Event.Enemy.WeakPoint.Hide\")"))))))

(event EventTick
  (params (DeltaSeconds :type Float%20%28single-precision%29))
  (|ShowDebugHealthText))

(fn ConstructionScript
  (Components|StaticMesh|SetStaticMesh (Variables|Default|GetMesh) (Variables|Setting|GetRegularMesh))
  (Rendering|Material|SetMaterial (Variables|Default|GetMesh) 0 (Variables|Setting|GetHiddenMaterial)))

(fn SetWeakPointStatus
  (params (Expose :type Boolean))
  ;[0.15 0.15 0.15 0.5] Temp; can be polished in the future
  (if Expose
    (Rendering|Material|SetMaterial (Variables|Default|GetMesh) 0 (Variables|Setting|GetExposedMaterial))
    (else
      (Rendering|Material|SetMaterial (Variables|Default|GetMesh) 0 (Variables|Setting|GetHiddenMaterial))))
  (return))

(fn StartDeathRoutine
  ;[0.15 0.15 0.15 0.5] VFX temp
  (Effects|SpawnEmitteratLocation "/Game/EngineDefault/StarterContent/Particles/P_Explosion.P_Explosion" (Transformation|GetActorLocation self) "0, 0, 0" "1.500000,1.500000,1.000000")
  ;[0.15 0.15 0.15 0.5] Change mesh
  (Components|StaticMesh|SetStaticMesh (Variables|Default|GetMesh) (Variables|Setting|GetDestroyedMesh))
  (Rendering|Material|SetMaterial (Variables|Default|GetMesh) 0 (Variables|Setting|GetDestroyedMaterial))
  (return))

(fn SetMaxHealth
  (params (MaxHealth :type Float%20%28double-precision%29))
  (bind _abilitysystemcomponent (Variables|Default|GetAbilitySystemComponent))
  (bind _returnvalue (Ability|GameplayEffect|AssignTagSetbyCallerMagnitude (GameplayEffects|MakeOutgoingSpec :self _abilitysystemcomponent :GameplayEffectClass "/Game/Enemy/GameplayEffects/GE_WeakPoint_MaxHealth.GE_WeakPoint_MaxHealth_C") "(TagName=\"SetByCaller.MaxHealth\")" MaxHealth))
  (GameplayEffects|ApplyGameplayEffectSpecToSelf _abilitysystemcomponent _returnvalue))