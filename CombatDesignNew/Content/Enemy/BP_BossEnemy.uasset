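; Boss enemy that takes damage through weak points and shows its health on a boss health bar widget.
; On BeginPlay it spawns a BP_WeakPoint at every socket of the boss mesh and sets max health through a SetByCaller gameplay effect.
; Weak point hit and destroy gameplay events apply a damage effect using the event magnitude.
; GAS health changes refresh the WB_Boss widget.
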(event OnHealthChange(GSCCore)
  (params (DeltaValue :type Float%20%28single-precision%29) (EventTags :type Gameplay%20Tag%20Container%20Structure))
  (bind _self self)
  ;[0.15 0.15 0.15 0.5] Update boss widget on health change
  (Default|UpdateHealthData (Variables|Default|GetBossWidget) (.ReturnValue (Ability|Attribute|GetFloatAttribute _self "(AttributeName=\"MaxHealth\",Attribute=/Script/GASCompanion.GSCAttributeSet:MaxHealth,AttributeOwner=\"/Script/CoreUObject.Class'/Script/GASCompanion.GSCAttributeSet'\")")) (.ReturnValue (Ability|Attribute|GetFloatAttribute _self "(AttributeName=\"Health\",Attribute=/Script/GASCompanion.GSCAttributeSet:Health,AttributeOwner=\"/Script/CoreUObject.Class'/Script/GASCompanion.GSCAttributeSet'\")"))))

(event EventBeginPlay
  (Utilities|FlowControl|Sequence
    (:then_0
      (CallFunction|SpawnWeakPointActors))
    (:then_1
      (CallFunction|SetMaxHealth (Variables|Setting|GetMaxHealth)))
    (:then_2
      ;[0.15 0.15 0.15 0.5] Take damage from weak points
      (|TakeDamageOnWeakPointHit)
      (|TakeDamageOnWeakPointDestroyed))
    (:then_3
      ;[0.15 0.15 0.15 0.5] Boss healthbar
      (bind _returnvalue (UserInterface|CreateWidget "/Game/UI/WB_Boss.WB_Boss_C" (Game|GetPlayerController 0)))
      (bind _output_get (Variables|Default|SetBossWidget _returnvalue))
      (UserInterface|Viewport|AddtoPlayerScreen _output_get)
      (|InitHealthDataForBossWidget))))

(fn ConstructionScript)

(fn SpawnWeakPointActors
  (bind _self self)
  (bind _output_get (Variables|WeakPoint|SetWeakPointSockets (Transformation|GetAllSocketNames (Variables|Default|GetTempBossMesh))))
  (for _array_element _output_get
    (bind _returnvalue (Game|SpawnActorfromClass "/Game/Enemy/WeakPoint/BP_WeakPoint.BP_WeakPoint_C" (Transformation|GetSocketTransform (Variables|Default|GetTempBossMesh) _array_element "RTS_World") "AlwaysSpawn" "OverrideRootScale" _self _self))
    (Transformation|AttachComponentToComponent _returnvalue (Variables|Default|GetTempBossMesh) _array_element "SnapToTarget" "SnapToTarget" "SnapToTarget" true)
    (Utilities|Map|Add (Variables|WeakPoint|GetWeakPoints) (Utilities|String|ToString(Name) _array_element) _returnvalue))
  (return))

(fn SetMaxHealth
  (params (MaxHealth :type Float%20%28double-precision%29))
  (bind _abilitysystemcomponent (Variables|Default|GetAbilitySystemComponent))
  (bind _returnvalue (Ability|GameplayEffect|AssignTagSetbyCallerMagnitude (GameplayEffects|MakeOutgoingSpec :self _abilitysystemcomponent :GameplayEffectClass "/Game/Enemy/GameplayEffects/GE_Boss_MaxHealth.GE_Boss_MaxHealth_C") "(TagName=\"SetByCaller.MaxHealth\")" MaxHealth))
  (GameplayEffects|ApplyGameplayEffectSpecToSelf _abilitysystemcomponent _returnvalue))