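; Golem boss enemy that takes damage through weak points and shows its health in an on-screen boss bar.
; On BeginPlay it spawns BP_WeakPoint actors on skeletal mesh sockets and creates the WB_Boss widget.
; Weak point hit and destroy gameplay events apply GE_Boss_Damage to the boss, passing the event magnitude as SetByCaller damage.
; GAS health change events refresh the widget.
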(event OnHealthChange(GSCCore)
  (params (DeltaValue :type Float%20%28single-precision%29) (EventTags :type Gameplay%20Tag%20Container%20Structure))
  (bind _self self)
  (Default|UpdateHealthData (Variables|Default|GetBossWidget) (.ReturnValue (Ability|Attribute|GetFloatAttribute _self "(AttributeName=\"MaxHealth\",Attribute=/Script/GASCompanion.GSCAttributeSet:MaxHealth,AttributeOwner=\"/Script/CoreUObject.Class'/Script/GASCompanion.GSCAttributeSet'\")")) (.ReturnValue (Ability|Attribute|GetFloatAttribute _self "(AttributeName=\"Health\",Attribute=/Script/GASCompanion.GSCAttributeSet:Health,AttributeOwner=\"/Script/CoreUObject.Class'/Script/GASCompanion.GSCAttributeSet'\")"))))

(event EventBeginPlay
  (Utilities|FlowControl|Sequence
    (:then_0
      (CallFunction|SpawnWeakpointActors))
    (:then_1
      ;[0.15 0.15 0.15 0.5] Boss healthbar
      (bind _returnvalue (UserInterface|CreateWidget "/Game/UI/WB_Boss.WB_Boss_C" (Game|GetPlayerController 0)))
      (bind _output_get (Variables|Default|SetBossWidget _returnvalue))
      (UserInterface|Viewport|AddtoPlayerScreen _output_get)
      (|InitHealthDataForBossWidget_2))
    (:then_2
      (|TakeDamageOnWeakPointHit_2)
      (|TakeDamageOnWeakPointDestroyed_2))))

(fn ConstructionScript)

(fn SpawnWeakpointActors
  (bind _self self)
  (for _array_element (Variables|Default|GetWeakPointSockets)
    (bind _returnvalue (Game|SpawnActorfromClass "/Game/Enemy/WeakPoint/BP_WeakPoint.BP_WeakPoint_C" (Math|Transform|MakeTransform (.location (Transformation|GetSocketTransform (Variables|Default|GetSK_Ancient_Golem_Moving_Wheels) _array_element "RTS_World")) (.rotation (Transformation|GetSocketTransform (Variables|Default|GetSK_Ancient_Golem_Moving_Wheels) _array_element "RTS_World")) "0.001000,0.001000,0.001000") "AlwaysSpawn" "OverrideRootScale" _self _self))
    (Transformation|AttachComponentToComponent _returnvalue (Variables|Default|GetSK_Ancient_Golem_Moving_Wheels) _array_element "SnapToTarget" "SnapToTarget" "SnapToTarget" true)
    (Utilities|Map|Add (Variables|Default|GetWeakPoints) (Utilities|String|ToString(Name) _array_element) _returnvalue)
    (Transformation|SetActorScale3D _returnvalue "2.500000,2.500000,2.500000")
    (Components|StaticMesh|SetStaticMesh (Variables|/Game/Enemy/WeakPoint/BP_WeakPoint.BP_WeakPoint_C|GetMesh _returnvalue) "/Game/EngineDefault/StarterContent/Props/MaterialSphere.MaterialSphere"))
  (return))