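; BP_Dummy is a dummy enemy actor that displays its health as floating text in the world.
; Every Tick it reads a float gameplay attribute from itself and writes it to a TextRender component as an HP label.
; The same Tick rotates the text to face the first player's camera, acting as a simple billboard.
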(event EventTick
  (params (DeltaSeconds :type Float%20%28single-precision%29))
  (Rendering|Components|TextRender|SetText (Variables|Default|GetTextRender) (Utilities|Text|FormatText "HP: {Health}" (.ReturnValue (Ability|Attribute|GetFloatAttribute self "(AttributeName=\"Health\",Attribute=/Script/GASCompanion.GSCAttributeSet:Health,AttributeOwner=\"/Script/CoreUObject.Class'/Script/GASCompanion.GSCAttributeSet'\")"))))
  (Transformation|SetWorldRotation (Variables|Default|GetTextRender) (Math|Rotator|FindLookatRotation (Transformation|GetWorldLocation (Variables|Default|GetTextRender)) (Camera|GetCameraLocation (Variables|/Script/Engine.PlayerController|GetPlayerCameraManager (Game|GetPlayerController 0)))) false false))

(fn ConstructionScript)