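; BP_FollowEnemy is a melee enemy that chases the player within a set distance and attacks on arrival.
; Tick drives AIMoveTo, whose success starts a charge effect, then briefly enables a sphere hitbox that launches the player and activates a GAS attack ability.
; GAS Companion events knock the enemy back on damage, print health changes and explode it on death.
; Capsule overlaps also check for fist hitboxes to trigger knockback.
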(event OnComponentBeginOverlap(Sphere)
  (params (OverlappedComponent :type Primitive%20Component%20Object%20Reference) (OtherActor :type Actor%20Object%20Reference) (OtherComp :type Primitive%20Component%20Object%20Reference) (OtherBodyIndex :type Integer) (bFromSweep :type Boolean) (SweepResult :type Hit%20Result%20Structure%20%28by%20ref%29))
  (if (Variables|Default|GetIsAttacking)
    (bind _asbp_player_character (Utilities|Casting|CastToBP_PlayerCharacter OtherActor))
    (Utilities|FlowControl|DoOnce false :!label _label
      (:Completed
        (Character|LaunchCharacter _asbp_player_character (* (Math|Vector|Normalize (- (Transformation|GetActorLocation _asbp_player_character) (Transformation|GetActorLocation))) (Variables|Default|GetKnockbackPower)) true true)
        (Abilities|TryActivateAbilitybyClass (Variables|Default|GetGSCAbilitySystem) "/Game/Enemy/FollowEnemy/GA_FollowEnemyAttack.GA_FollowEnemyAttack_C" true)
        (Utilities|FlowControl|Delay 0.5)
        (goto _label Reset)))))

(event OnDamage(GSCCore)
  (params (DamageAmount :type Float%20%28single-precision%29) (SourceCharacter :type Actor%20Object%20Reference) (DamageTags :type Gameplay%20Tag%20Container%20Structure%20%28by%20ref%29))
  (CallFunction|TakeKnockback SourceCharacter))

(event OnDeath(GSCCore)
  (Effects|SpawnEmitteratLocation "/Game/EngineDefault/StarterContent/Particles/P_Explosion.P_Explosion" (Transformation|GetActorLocation))
  (Utilities|FlowControl|Delay 0.2)
  (Actor|DestroyActor))

(event OnComponentBeginOverlap(CapsuleComponent)
  (params (OverlappedComponent :type Primitive%20Component%20Object%20Reference) (OtherActor :type Actor%20Object%20Reference) (OtherComp :type Primitive%20Component%20Object%20Reference) (OtherBodyIndex :type Integer) (bFromSweep :type Boolean) (SweepResult :type Hit%20Result%20Structure%20%28by%20ref%29))
  (bind _returnvalue (Utilities|GetObjectName OverlappedComponent))
  (if (or (Utilities|Enum|Equal(Enum) _returnvalue "FistHitboxR") (Utilities|Enum|Equal(Enum) _returnvalue "FistHitboxL"))
    (CallFunction|TakeKnockback)))

(event OnHealthChange(GSCCore)
  (params (DeltaValue :type Float%20%28single-precision%29) (EventTags :type Gameplay%20Tag%20Container%20Structure))
  (Development|PrintString (Utilities|String|ToString(Float) (Class|GSCCoreComponent|GetHealth (Variables|Default|GetGSCCore)))))

(event Custom|ExecuteAttack
  (bind _sphere (Variables|Default|GetSphere))
  (bind _sphere_2 (Variables|Default|GetSphere))
  (Variables|Default|SetIsAttacking true)
  (Niagara|SpawnSystemAttached "/Game/Enemy/FollowEnemy/NS_EnemyCharge.NS_EnemyCharge" (Variables|Collision|GetCapsuleComponent) "None" "0, 0, 0" "0, 0, 0" "KeepRelativeOffset" true)
  (Utilities|FlowControl|Delay 0.75)
  (Development|SetHiddeninGame _sphere false false)
  (Collision|SetCollisionEnabled _sphere "QueryOnly")
  (Utilities|FlowControl|Delay 0.5)
  (Development|SetHiddeninGame _sphere_2 true false)
  (Collision|SetCollisionEnabled _sphere_2 "NoCollision")
  (Variables|Default|SetIsAttacking false))

(event Custom|TakeKnockback
  (params (Source :type Actor%20Object%20Reference))
  (Character|LaunchCharacter (* (Math|Vector|Normalize (- (Transformation|GetActorLocation) (Transformation|GetActorLocation Source))) (Variables|Default|GetKnockbackPower)) true true))

(event EventBeginPlay
  (bind _returnvalue (Actor|GetActorOfClass "/Game/Player/BP_PlayerCharacter.BP_PlayerCharacter_C"))
  (Variables|Default|SetPlayer _returnvalue)
  (Collision|SetCollisionEnabled (Variables|Default|GetSphere) "NoCollision"))

(event EventTick
  (params (DeltaSeconds :type Float%20%28single-precision%29))
  (if (not (Variables|Default|GetIsAttacking))
    (bind _isinrange (CallFunction|IsinAttackRange))
    (if _isinrange
      (AI|AIMoveTo self "0, 0, 0" (Variables|Default|GetPlayer) 75.0 false
        (:OnSuccess
          (CallFunction|ExecuteAttack))))))

(fn ConstructionScript)

(fn IsinAttackRange
  (return (< (Math|Vector|Distance(Vector) (Transformation|GetActorLocation (Variables|Default|GetPlayer)) (Transformation|GetActorLocation)) (Variables|Default|GetChase%20Distance))))