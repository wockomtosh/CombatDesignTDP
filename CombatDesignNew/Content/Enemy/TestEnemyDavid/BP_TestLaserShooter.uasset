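; BP_TestLaserShooter is a test enemy actor that turns to face the player; the graphs contain no firing logic.
; BeginPlay caches the first player pawn, and Tick rotates the root component toward it using RInterpTo for a lagged follow.
; The Delay variable feeds the interpolation speed, so higher values track faster.
; An unconnected alternative that snaps instantly to the player remains in the graph.
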(event EventBeginPlay
  (Variables|Default|SetCharacter (Game|Player|GetPlayerPawn 0)))

(event EventTick
  (params (DeltaSeconds :type Float%20%28single-precision%29))
  ;[0.15 0.15 0.15 0.5] Look at Player in realtime with a delay
  (Transformation|SetWorldRotation (Variables|Default|GetDefaultSceneRoot) (Math|Interpolation|RInterpTo (Transformation|GetWorldRotation (Variables|Default|GetDefaultSceneRoot)) (Math|Rotator|FindLookatRotation (Transformation|GetActorLocation) (Transformation|GetActorLocation (Variables|Default|GetCharacter))) (Utilities|Time|GetWorldDeltaSeconds) (Variables|Default|GetDelay)) false false))

(fn ConstructionScript)