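; Enemy turret that tracks the player and fires a lightning strike after a targeting countdown.
; Each Tick polls a perception check; while active, it rotates toward the player, then after a delay activates GA_LightningStrike through GAS and resets.
; Cylinder material shows idle, targeting and warning states, with a sound at the warning threshold and an optional debug cone.
; The sphere-trace FireLaser event is obsolete, replaced by the ability.
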(event Custom|FireLaser
  ;[0.15 0.15 0.15 0.5] Obsolete (replaced by GA_LightningStrike)
  (bind _showtraces (Class|BPIController|GetDebugInfo(Message) (Game|GetPlayerController 0)))
  (bind _outactors (Actor|GetAllActorsOfClass "/Game/Enemy/BP_Enemy_GolemBoss.BP_Enemy_GolemBoss_C"))
  (bind (_start _end) (CallFunction|GetTraceParameters))
  (bind (_outhit _returnvalue) (Collision|SphereTraceByChannel _start _end (Variables|Setting|GetDamageRadius) "TraceTypeQuery2" false _outactors (select _showtraces "ForDuration" "None") true "(R=1.000000,G=0.000000,B=0.000000,A=1.000000)" "(R=0.000000,G=1.000000,B=0.000000,A=1.000000)" 0.5))
  (if _returnvalue
    (Utilities|FlowControl|Sequence
      (:then_0
        (Niagara|SpawnSystematLocation "/Game/Vefects/Zap_VFX/VFX/Zap/Particles/NS_Zap_01_Red_Custom.NS_Zap_01_Red_Custom" (.ImpactPoint (Collision|BreakHitResult _outhit)) (Math|Rotator|MakeRotator (.roll (Math|Rotator|FindLookatRotation (.ImpactPoint (Collision|BreakHitResult _outhit)) (Transformation|GetWorldLocation (Variables|Default|GetTurret)))) (+ (.pitch (Math|Rotator|FindLookatRotation (.ImpactPoint (Collision|BreakHitResult _outhit)) (Transformation|GetWorldLocation (Variables|Default|GetTurret)))) -9e+01) (.yaw (Math|Rotator|FindLookatRotation (.ImpactPoint (Collision|BreakHitResult _outhit)) (Transformation|GetWorldLocation (Variables|Default|GetTurret))))) "3.000000,3.000000,1.000000")
        (Effects|SpawnEmitteratLocation "/Game/EngineDefault/StarterContent/Particles/P_Explosion.P_Explosion" (.ImpactPoint (Collision|BreakHitResult _outhit)) "0, 0, 0" "2.000000,2.000000,2.000000")
        (Audio|SpawnSoundatLocation "/Game/Vefects/Zap_VFX/Audio/SFX_Vefects_Zap_Small_01_Cue.SFX_Vefects_Zap_Small_01_Cue" (.ImpactPoint (Collision|BreakHitResult _outhit)) "0, 0, 0" 1.0 1.0 0.0 0 0))
      (:then_1
        (Ability|SendGameplayEventtoActor)))))

(event Custom|TargetPlayer
  (bind (_start _end) (Utilities|TraceParameters))
  (CallFunction|RotatetoTarget (Variables|Default|GetTargetActor) (Variables|Setting|GetTargetFollowSpeed))
  (bind _showtraces (Class|BPIController|GetDebugInfo(Message) (Game|GetPlayerController 0)))
  (Collision|LineTraceByChannel _start _end "TraceTypeQuery1" false 0 "ForOneFrame" true "(R=1.000000,G=0.000000,B=0.000000,A=1.000000)" "(R=0.000000,G=0.000000,B=0.000000,A=1.000000)" 0.2))

(event EventTick
  (params (DeltaSeconds :type Float%20%28single-precision%29))
  (bind _perceptionangle (Variables|Setting|GetPerceptionAngle))
  (Utilities|FlowControl|Sequence
    (:then_0
      (Variables|Default|SetIsActive (Utilities|GetPerceptionIsActive)))
    (:then_1
      (bind _showtraces (Class|BPIController|GetDebugInfo(Message) (Game|GetPlayerController 0)))
      (if _showtraces
        (Class|KismetSystemLibrary|DrawDebugConeinDegrees (Transformation|GetActorLocation) (Transformation|GetActorForwardVector) (Variables|Setting|GetPerceptionRange) _perceptionangle _perceptionangle 12 (Math|Color|SelectColor "(R=1.000000,G=0.018362,B=0.000000,A=1.000000)" "(R=0.097575,G=1.000000,B=0.000000,A=1.000000)" (Variables|Default|GetIsActive)) 0.0 0.0)))
    (:then_2
      (Rendering|Material|SetMaterial (Variables|Default|GetCylinder) 0 (select (Variables|Default|GetIsActive) (select (< (- (Variables|Setting|GetTargetDuration) (Variables|Default|GetTargetTimer)) (Variables|Setting|GetWarningThreshold)) "/Game/Material/M_Emissive_Red.M_Emissive_Red" "/Game/Material/M_Emissive_Yellow.M_Emissive_Yellow") "/Game/Material/M_Emissive_Blue.M_Emissive_Blue")))
    (:then_3
      (if (Variables|Default|GetIsActive)
        (Development|PrintString (Utilities|String|ToString(Text) (Utilities|Text|ToText(Float) (- (Variables|Setting|GetTargetDuration) (Variables|Default|GetTargetTimer)) "HalfToEven" false true 1 324 0 2)) true true "(R=0.000000,G=0.660000,B=1.000000,A=1.000000)" 0.0)
        (if (< (Variables|Default|GetTargetTimer) (Variables|Setting|GetTargetDuration))
          (CallFunction|TargetPlayer)
          (Variables|Default|SetTargetTimer (+ (Variables|Default|GetTargetTimer) (Utilities|Time|GetWorldDeltaSeconds)))
          (else
            (Utilities|FlowControl|Delay (Variables|Setting|GetFireDelay))
            (Abilities|TryActivateAbilitybyClass (Variables|Default|GetGSCAbilitySystem) "/Game/Enemy/Turret/GA_LightningStrike.GA_LightningStrike_C" true)
            (Variables|Default|SetTargetTimer 0.0)))
        (else
          (Variables|Default|SetTargetTimer 0.0))))
    (:then_4
      (if (Math|Float|NearlyEqual(Float) (- (Variables|Setting|GetTargetDuration) (Variables|Default|GetTargetTimer)) (Variables|Setting|GetWarningThreshold) 0.01)
        (Audio|PlaySound2D "/Engine/VREditor/Sounds/UI/Enter_Simulate.Enter_Simulate" 1.0 1.0 0.0 0 0)))))

(event EventBeginPlay
  (Utilities|FlowControl|Sequence
    (:then_0
      (Variables|Default|SetTargetActor (Game|GetPlayerCharacter 0)))))

(fn ConstructionScript)

(fn RotatetoTarget
  (params (TargetActor :type Actor%20Object%20Reference) (InterpSpeed :type Float%20%28double-precision%29))
  (bind _turret (Variables|Default|GetTurret))
  (Transformation|SetWorldRotation _turret (Math|Interpolation|RInterpTo (Transformation|GetWorldRotation _turret) (Math|Rotator|FindLookatRotation (Transformation|GetWorldLocation _turret) (Transformation|GetActorLocation TargetActor)) (Utilities|Time|GetWorldDeltaSeconds) InterpSpeed) false false))

(fn GetTraceParameters
  (bind _returnvalue (Transformation|GetActorLocation))
  (return _returnvalue (+ _returnvalue (* (Math|Vector|GetForwardVector (Variables|Default|GetTurret)) (Variables|Setting|GetPerceptionRange)))))